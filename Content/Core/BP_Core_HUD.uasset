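; Core HUD Blueprint that spawns the main HUD widget and the in-game inventory and equipment menus on BeginPlay.
; Menus are kept in a list, and ToggleWidget shows or hides the requested one while collapsing any other visible menu.
; Opening a menu switches to Game and UI input with the cursor shown, and closing it restores game-only input with the cursor hidden.
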(event `self.ReceiveBeginPlay`
  ; Focus Input on game
  (`WidgetBlueprintLibrary.SetInputMode_GameOnly` (`self.GetOwningPlayerController`))
  ; Game
  (`self.CreateGameWidgets`)
  ; Game Menus
  (`self.CreateGameMenuWidgets`))

(fn `CreateGameMenuWidgets`
  (`|ExecutionSequence`
    (:`then_0`
      (`|ExecutionSequence`
        (:`then_0`
          (bind _returnvalue (`|CreateWidget` "/Game/Widgets/InGame/Menus/WBP_InGame_Inventory.WBP_InGame_Inventory_C" (`self.GetOwningPlayerController`)))
          (bind _output_get (set `self.WBP_InGame_Inventory` _returnvalue))
          (`KismetArrayLibrary.Array_Add` (`self.GameMenu_WidgetLists`) _output_get))
        (:`then_1`
          (bind _returnvalue_2 (`|CreateWidget` "/Game/Widgets/InGame/Menus/WBP_InGame_Equipment.WBP_InGame_Equipment_C" (`self.GetOwningPlayerController`)))
          (bind _output_get_2 (set `self.WBP_InGame_Equipment` _returnvalue_2))
          (`KismetArrayLibrary.Array_Add` (`self.GameMenu_WidgetLists`) _output_get_2))))
    (:`then_1`
      (for _array_element (`self.GameMenu_WidgetLists`)
        (`UserWidget.AddToViewport` _array_element 0)))))

(fn `CreateGameWidgets`
  (bind _returnvalue (`|CreateWidget` "/Game/Widgets/InGame/WBP_Core_HUD.WBP_Core_HUD_C" (`self.GetOwningPlayerController`)))
  (bind _output_get (set `self.WBP_Core_HUD` _returnvalue))
  (`UserWidget.AddToViewport` _output_get 0))

(fn `FocusGame`
  (bind _returnvalue (`self.GetOwningPlayerController`))
  (`Widget.SetVisibility` (`self.WidgetToFocus`) "Collapsed")
  (`WidgetBlueprintLibrary.SetInputMode_GameOnly` _returnvalue)
  (set `PlayerController.bShowMouseCursor` false _returnvalue))

(fn `FocusWidget`
  (bind _returnvalue (`self.GetOwningPlayerController`))
  (`Widget.SetVisibility` (`self.WidgetToFocus`) "SelfHitTestInvisible")
  (`WidgetBlueprintLibrary.SetInputMode_GameAndUIEx` _returnvalue (`self.WidgetToFocus`))
  (set `PlayerController.bShowMouseCursor` true _returnvalue))

(fn `ToggleEquipment`
  (`self.ToggleWidget` (`self.WBP_InGame_Equipment`)))

(fn `ToggleInventory`
  (`self.ToggleWidget` (`self.WBP_InGame_Inventory`)))

(fn `ToggleWidget`
  (params (TargetWidget :type "UserWidget Object Reference"))
  (`/Engine/EditorBlueprintResources/StandardMacros.IsValid` TargetWidget
    (:`Is Valid`
      (set `self.WidgetToFocus` TargetWidget)
      (for _array_element (`self.GameMenu_WidgetLists`)
        (`/Engine/EditorBlueprintResources/StandardMacros.IsValid` _array_element
          (:`Is Valid`
            (if (== (`self.WidgetToFocus`) _array_element)
              (if (`Widget.IsVisible` (`self.WidgetToFocus`))
                (`self.FocusGame`)
                (else
                  (`self.FocusWidget`)))
              (elif (`Widget.IsVisible` _array_element)
                (`Widget.SetVisibility` _array_element "Collapsed")))))))))

(fn `UserConstructionScript`)